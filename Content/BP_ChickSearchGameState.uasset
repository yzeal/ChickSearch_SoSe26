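; BP_ChickSearchGameState tracks the player's progress in a game about collecting chicks and decides when the game is won.
; On BeginPlay it counts all BP_Chick actors in the level as the total.
; The AddChick event increments the collected count; when it matches the total, it sets GameWon, switches player 0 to UI-only input and shows the mouse cursor.
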(event Custom|AddChick
  (bind _returnvalue (Game|GetPlayerController 0))
  ;[0.15 0.15 0.15 0.5] Küken aufsammeln
  (Variables|Default|SetCollectedChickNumber (+ (Variables|Default|GetCollectedChickNumber) 1))
  ;[0.15 0.15 0.15 0.5] prüfen, ob alle Küken aufgesammelt sind
  (if (== (Variables|Default|GetCollectedChickNumber) (Variables|Default|GetTotalChickNumber))
    (Variables|Default|SetGameWon true)
    (Input|SetInputModeUIOnly _returnvalue 0 "DoNotLock" false)
    (Variables|/Script/Engine.PlayerController|SetbShowMouseCursor _returnvalue true)))

(event EventBeginPlay
  ;[0.15 0.15 0.15 0.5] Küken im Level zählen
  (bind _outactors (Actor|GetAllActorsOfClass "/Game/Characters/Chick/BP_Chick.BP_Chick_C"))
  (Variables|Default|SetTotalChickNumber (Utilities|Array|Length _outactors)))

(fn ConstructionScript)